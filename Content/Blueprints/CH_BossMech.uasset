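; Boss mech character with a child-actor gatling gun, a material-driven health bar and a staged explosive defeat.
; On BeginPlay it caches the gun and creates the dynamic bar material that Tick feeds with health percentage.
; ABP_Boss calls the gatling engage and disengage events.
; Defeat unpossesses, plays the explode montage and pitch-shifts audio; a delayed event scatters bones with random impulses, spawns the explosion, then calls the parent's defeat.
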(event Custom|StartDelayedDefeat
  (bind _mesh (Variables|Character|GetMesh))
  (bind _returnvalue (Transformation|GetSocketTransform _mesh "Cockpit_joint" "RTS_World"))
  (Class|BaseCharacter|StartDelayedIsDefeatedProcedure)
  (for _array_element (Transformation|GetAllSocketNames (Variables|Character|GetMesh))
    (Physics|AddImpulse (Variables|Character|GetMesh) (* (Math|Random|RandomUnitVector) 1.5e+03) _array_element true)
    (Class|PrimitiveComponent|AddAngularImpulseinDegrees (Variables|Character|GetMesh) (* (Math|Random|RandomUnitVector) (* (Math|Random|RandomFloatinRange -1.0 1.0) 5e+02)) _array_element true))
  (Effects|SpawnEmitteratLocation "/Game/Effects/Particles/Explosions/p_explosion.p_explosion" (.location _returnvalue) (.rotation _returnvalue) "0.500000,0.500000,0.500000")
  (Audio|PlaySoundatLocation "/Game/MigratedContent/MigratedAudio/StarterContentSounds/S_Explosion01.S_Explosion01" (.location _returnvalue) "0, 0, 0" 1.0 1.0 0.0 "/Game/MigratedContent/MigratedAudio/LevelSoundAttenuation.LevelSoundAttenuation" 0 0)
  (Utilities|FlowControl|Delay 2.0)
  (|CallParentFunction))

(event Custom|EventEndGatling
  ;[0.2384 0.491 1] Main logic, setting references and events
  ;;[1 1 1] Start/End gatling gun - called from ABP_Boss
  (Default|Disengage (Variables|Default|GetGatling)))

(event Custom|EventStartGatling
  ;[0.2384 0.491 1] Main logic, setting references and events
  ;;[1 1 1] Start/End gatling gun - called from ABP_Boss
  (Variables|Default|SetEngageGatling true)
  (Default|Engage (Variables|Default|GetGatling)))

(event EventBeginPlay
  (bind _healthbar (Variables|Default|GetHealthBar))
  ;[0.2384 0.491 1] Main logic, setting references and events
  ;;[1 1 1] Set references and start behavior tree
  (bind _asbp_gatling_gun (Utilities|Casting|CastToBP_GatlingGun (Variables|/Script/Engine.ChildActorComponent|GetChildActor (Variables|Default|GetGatlingGun))))
  (Variables|Default|SetGatling _asbp_gatling_gun)
  (CallFunction|GetBehavior)
  ;;[1 1 1] Creating and updating health bar
  (bind _returnvalue (Rendering|Material|CreateDynamicMaterialInstance _healthbar 0 (Rendering|Material|GetMaterial _healthbar 0) "None" :!class /Script/Engine.PrimitiveComponent))
  (bind _output_get (Variables|Default|SetCurrentHealthBar _returnvalue))
  (Variables|Default|SetbHealthBarSetup true))

(event EventEventIsDefeated
  (bind _audio (Variables|Default|GetAudio))
  (Pawn|UnPossess (Pawn|GetController))
  (bind _returnvalue (Animation|GetCurrentMontage :!class /Script/Engine.Character))
  (Animation|StopAnimMontage _returnvalue)
  (Animation|PlayAnimMontage "/Game/Meshes/Characters/Boss/BossExplode_Montage.BossExplode_Montage" 1.0 "None")
  (Audio|Components|Audio|SetVolumeMultiplier _audio 1.0 :!class /Script/Engine.AudioComponent)
  (bind _pitch (Timeline|PitchEnd PlayFromStart)
    (:Update
      (Audio|Components|Audio|SetPitchMultiplier _audio _pitch))
    (:Finished
      (Audio|Components|Audio|FadeOut _audio 1.0 0.0 "Linear" :!class /Script/Engine.AudioComponent))))

(event EventTick
  (params (DeltaSeconds :type Float%20%28single-precision%29))
  ;[0.2384 0.491 1] Main logic, setting references and events
  ;;[1 1 1] Creating and updating health bar
  (if (Variables|Default|GetbHealthBarSetup)
    (Rendering|Material|SetScalarParameterValue (stale EventBeginPlay _output_get) "HealthPointPercentage" (/ (Variables|Default|GetcurrentHealthPoints) (Variables|Default|GetmaxHealthPoints)) :!class /Script/Engine.MaterialInstanceDynamic)))

(fn ConstructionScript)

(fn GetBehavior
  (return "NewEnumerator0"))