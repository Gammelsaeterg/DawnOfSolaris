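; BP_BossClaw is a boss claw weapon Blueprint whose only logic of its own is a hit-effect event.
; DebugSpawnHitFX plays the Hit2 sound with randomized pitch and level attenuation at a given location, and spawns the RobotSplat emitter there.
; Sound volume scales with the SoundVolume setting read from BP_DefaultGameInstance.
; BeginPlay, overlap and Tick are disabled stubs, and the construction script only calls its parent.
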(event EventBeginPlay
  (|CallParentFunction) ; This node is disabled and will not be called.\nDrag off pins to build functionality.
)

(event Collision|EventActorBeginOverlap
  (params (OtherActor :type Actor%20Object%20Reference))
  (|CallParentFunction OtherActor) ; This node is disabled and will not be called.\nDrag off pins to build functionality.
)

(event EventTick
  (params (DeltaSeconds :type Float%20%28single-precision%29))
  (|CallParentFunction DeltaSeconds) ; This node is disabled and will not be called.\nDrag off pins to build functionality.
)

(event EventDebugSpawnHitFX
  (params (location :type Vector :default "0, 0, 0"))
  (Audio|PlaySoundatLocation "/Game/Sound/PlaceholderSounds/hit2.hit2" location "0, 0, 0" (/ (Variables|/Script/DawnOfSolaris.MainGameInstance|GetsoundVolume (.AsBP%20Default%20Game%20Instance (Utilities|Casting|CastToBP_DefaultGameInstance (Game|GetGameInstance)))) 1e+02) (Math|Random|RandomFloatinRange 0.7 1.3) 0.0 "/Game/MigratedContent/MigratedAudio/LevelSoundAttenuation.LevelSoundAttenuation" 0 0)
  (Effects|SpawnEmitteratLocation "/Game/Particles/PlaceholderParticles/RobotSplat.RobotSplat" location))

(fn ConstructionScript
  (|CallParentFunction))