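; BP_GruntRifleProjectile is the grunt rifle projectile, handling its trail and hit effects.
; On BeginPlay it scales the Niagara trail width by average actor scale and caches the mesh material's EmissiveColor.
; DebugSpawnHitFX spawns an inactive burst system, sets its scaled size and cached color before activating it, plays a pitch-randomized, volume-scaled sound, and stops trail spawning.
; Mesh override and spin logic are left disconnected.
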(event EventBeginPlay
  (bind _returnvalue (Transformation|GetActorScale3D))
  (|CallParentFunction)
  (Niagara|SetNiagaraVariable(Float) (Variables|Default|GetProjectileTrails) "User.TrailWidth" (* (Variables|Default|GetdefaultTrailWidth) (/ (+ (.x _returnvalue) (.y _returnvalue) (.z _returnvalue)) 3.0)))
  (bind _returnvalue_2 (Rendering|Material|CreateDynamicMaterialInstance (Variables|Default|GetProjectileMesh) 0 (Rendering|Material|GetMaterial (Variables|Default|GetProjectileMesh) 0) "None" :!class /Script/Engine.PrimitiveComponent))
  (bind _returnvalue_3 (Rendering|Material|GetVectorParameterValue _returnvalue_2 "EmissiveColor" :!class /Script/Engine.MaterialInstanceDynamic))
  (Variables|Default|SetProjectileColor _returnvalue_3))

(event Collision|EventActorBeginOverlap
  (params (OtherActor :type Actor%20Object%20Reference))
  (|CallParentFunction OtherActor) ; This node is disabled and will not be called.\nDrag off pins to build functionality.
)

(event EventTick
  (params (DeltaSeconds :type Float%20%28single-precision%29))
  (|CallParentFunction DeltaSeconds))

(event EventDebugSpawnHitFX
  (params (location :type Vector :default "0, 0, 0"))
  (bind _returnvalue (Transformation|GetActorScale3D))
  (bind _returnvalue_2 (Niagara|SpawnSystematLocation "/Game/Particles/Niagara/AlienBurst/NS_AlienMeshBurst.NS_AlienMeshBurst" location "0, 0, 0" "1.000000,1.000000,1.000000" true false))
  (Niagara|SetNiagaraVariable(Float) _returnvalue_2 "User.CustomSpriteSize" (* (Variables|Default|GetdefaultHitEmitterSize) (/ (+ (.x _returnvalue) (.y _returnvalue) (.z _returnvalue)) 3.0)))
  (Niagara|SetNiagaraVariable(LinearColor) _returnvalue_2 "User.CustomColor" (Variables|Default|GetProjectileColor))
  (Components|Activation|Activate _returnvalue_2 false)
  (Audio|PlaySoundatLocation "/Game/Sound/PlaceholderSounds/whack1.whack1" location "0, 0, 0" (/ (Variables|/Script/DawnOfSolaris.MainGameInstance|GetsoundVolume (.AsBP%20Default%20Game%20Instance (Utilities|Casting|CastToBP_DefaultGameInstance (Game|GetGameInstance)))) 1e+02) (Math|Random|RandomFloatinRange 0.85 1.15) 0.0 "/Game/MigratedContent/MigratedAudio/LevelSoundAttenuation.LevelSoundAttenuation" "/Game/MigratedContent/MigratedAudio/DefaultSoundConcurrency.DefaultSoundConcurrency" 0)
  (Niagara|SetNiagaraVariable(Float) (Variables|Default|GetProjectileTrails) "User.TrailSpawnRate" 0.0))

(fn ConstructionScript
  (|CallParentFunction))