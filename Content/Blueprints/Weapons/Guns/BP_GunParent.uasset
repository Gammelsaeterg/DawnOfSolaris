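; BP_GunParent is a gun Blueprint, named as a parent class, that provides a basic hitscan shot.
; StartShooting sets IsFiring and calls FireBullet once, while StopShooting only clears the flag, so there is no repeat fire.
; FireBullet line-traces on the Visibility channel from BarrelRefpoint along its forward vector for Range.
; The shot only draws debug and prints a message; the hit result is not used.
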(event Custom|StartShooting
  (Variables|Default|SetIsFiring true)
  (CallFunction|FireBullet))

(event Custom|StopShooting
  (Variables|Default|SetIsFiring false))

(fn ConstructionScript)

(fn FireBullet
  (bind _barrel_refpoint (Variables|Default|GetBarrel_refpoint))
  (bind _returnvalue (Transformation|GetWorldLocation _barrel_refpoint))
  (Collision|LineTraceByChannel _returnvalue (+ _returnvalue (* (Math|Vector|GetForwardVector (Transformation|GetWorldRotation _barrel_refpoint)) (Variables|Default|GetRange))) "TraceTypeQuery1" false 0 "ForDuration")
  (Development|PrintString "HITSCAN"))