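; BP_AmbientAudio plays ambient sound that fades in when play begins and can be faded out on demand.
; On BeginPlay it scales the audio component's volume by the SoundVolume setting from BP_DefaultGameInstance, then fades in on a logarithmic curve.
; A FadeOutAudio function fades the component to silence with the same curve, for callers to invoke.
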(event EventBeginPlay
  (bind _asbp_default_game_instance (Utilities|Casting|CastToBP_DefaultGameInstance (Game|GetGameInstance)))
  (Audio|Components|Audio|SetVolumeMultiplier (Variables|Components|GetAudioComponent) (/ (Variables|/Script/DawnOfSolaris.MainGameInstance|GetsoundVolume _asbp_default_game_instance) 1e+02) :!class /Script/Engine.AudioComponent)
  (Audio|Components|Audio|FadeIn (Variables|Components|GetAudioComponent) 3.0 1.0 0.0 "Logarithmic" :!class /Script/Engine.AudioComponent))

(event EventTick
  (params (DeltaSeconds :type Float%20%28single-precision%29)))

(fn ConstructionScript)

(fn FadeOutAudio
  (Audio|Components|Audio|FadeOut (Variables|Components|GetAudioComponent) 3.0 0.0 "Logarithmic" :!class /Script/Engine.AudioComponent))