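; Alien player character Blueprint that records its controller ID on possession and adds debug visuals for melee attacks.
; When debug display is on, Tick shows the limb box matching the current hitbox type while an attack is active, using a DoOnce that resets once it ends.
; Debug events spawn hit splats and attach a wind-up fire effect to that limb, which Tick scales with charge amount.
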(event EventBeginPlay)

(event EventPossessed
  (params (NewController :type Controller%20Object%20Reference))
  ;[1 1 1] SetPlayerIndex
  (bind _asplayer_controller (Utilities|Casting|CastToPlayerController NewController))
  (Variables|Default|SetcurrentPlayerID (Class|GameplayStatics|GetPlayerControllerID _asplayer_controller)))

(event EventTick
  (params (DeltaSeconds :type Float%20%28single-precision%29))
  ;[1 1 1] Debug functions
  (if (Variables|Default|GetShowDebugHitboxes)
    (CallFunction|DrawDebugHitboxes)
    (CallFunction|ScaleFX)))

(event Collision|EventActorBeginOverlap
  (params (OtherActor :type Actor%20Object%20Reference)))

(event Custom|ResetDoOnceDebug
  (bind _currentattackhitboxtype (Variables|Default|GetcurrentAttackHitboxType))
  (bind _lefthanddebugbox (Variables|Default|GetLeftHandDebugBox))
  (bind _righthanddebugbox (Variables|Default|GetRightHandDebugBox))
  (bind _leftfootdebugbox (Variables|Default|GetLeftFootDebugBox))
  (bind _rightfootdebugbox (Variables|Default|GetRightFootDebugBox))
  (bind _leftkneedebugbox (Variables|Default|GetLeftKneeDebugBox))
  (bind _rightkneedebugbox (Variables|Default|GetRightKneeDebugBox))
  (bind _array (Utilities|Array|MakeArray _lefthanddebugbox _righthanddebugbox _leftfootdebugbox _rightfootdebugbox _leftkneedebugbox _rightkneedebugbox))
  (bind _output (Utilities|Array|Get(acopy) _array))
  (bind _output_2 (Utilities|Array|Get(acopy) _array 1))
  (bind _output_3 (Utilities|Array|Get(acopy) _array 2))
  (bind _output_4 (Utilities|Array|Get(acopy) _array 3))
  (bind _output_5 (Utilities|Array|Get(acopy) _array 4))
  (bind _output_6 (Utilities|Array|Get(acopy) _array 5))
  (bind _returnvalue (Utilities|Select :Index _currentattackhitboxtype :Default 0 :HeldObject 0 :Projectile 0 :LeftHand _output :LeftElbow 0 :LeftKnee _output_5 :LeftFoot _output_3 :RightHand _output_2 :RightElbow 0 :RightKnee _output_6 :RightFoot _output_4))
  ;[1 1 1] Debug hitbox
  (Utilities|FlowControl|DoOnce false) ; enters at Reset
)

(event Custom|DrawDebugHitboxes
  (bind _currentattackhitboxtype (Variables|Default|GetcurrentAttackHitboxType))
  (bind _lefthanddebugbox (Variables|Default|GetLeftHandDebugBox))
  (bind _righthanddebugbox (Variables|Default|GetRightHandDebugBox))
  (bind _leftfootdebugbox (Variables|Default|GetLeftFootDebugBox))
  (bind _rightfootdebugbox (Variables|Default|GetRightFootDebugBox))
  (bind _leftkneedebugbox (Variables|Default|GetLeftKneeDebugBox))
  (bind _rightkneedebugbox (Variables|Default|GetRightKneeDebugBox))
  (bind _array (Utilities|Array|MakeArray _lefthanddebugbox _righthanddebugbox _leftfootdebugbox _rightfootdebugbox _leftkneedebugbox _rightkneedebugbox))
  (bind _output (Utilities|Array|Get(acopy) _array))
  (bind _output_2 (Utilities|Array|Get(acopy) _array 1))
  (bind _output_3 (Utilities|Array|Get(acopy) _array 2))
  (bind _output_4 (Utilities|Array|Get(acopy) _array 3))
  (bind _output_5 (Utilities|Array|Get(acopy) _array 4))
  (bind _output_6 (Utilities|Array|Get(acopy) _array 5))
  (bind _returnvalue (Utilities|Select :Index _currentattackhitboxtype :Default 0 :HeldObject 0 :Projectile 0 :LeftHand _output :LeftElbow 0 :LeftKnee _output_5 :LeftFoot _output_3 :RightHand _output_2 :RightElbow 0 :RightKnee _output_6 :RightFoot _output_4))
  ;[1 1 1] Debug hitbox
  (if (Variables|Default|GetbAttackHitboxActive)
    (Utilities|FlowControl|DoOnce false
      (:Completed
        (Utilities|IsValid _returnvalue
          (:Is%20Valid
            (Rendering|SetVisibility _returnvalue true false)))))
    (else
      (for _array_element (Utilities|Array|MakeArray (Variables|Default|GetLeftHandDebugBox) (Variables|Default|GetRightHandDebugBox) (Variables|Default|GetLeftFootDebugBox) (Variables|Default|GetRightFootDebugBox) (Variables|Default|GetLeftKneeDebugBox) (Variables|Default|GetRightKneeDebugBox))
        (Rendering|SetVisibility _array_element false false))
      (CallFunction|ResetDoOnceDebug))))

(event Custom|ScaleFX
  (bind _tickwindupchargeamount (Variables|Default|GettickWindUpChargeAmount))
  (bind _returnvalue (* _tickwindupchargeamount 0.2))
  (bind _returnvalue_2 (+ _returnvalue 0.3))
  ;[1 1 1] Debug particle
  (bind _debugwindupfx (Variables|Default|GetDebugWindUpFX)
    (:then
      (Transformation|SetWorldScale3D _debugwindupfx (Math|Vector|MakeVector _returnvalue_2 _returnvalue_2 _returnvalue_2)))
    (:else)))

(event EventDebugSpawnHitFX
  (params (hitLocation :type Vector :default "0, 0, 0"))
  ;[1 1 1] Debug particle
  (Effects|SpawnEmitteratLocation "/Game/Particles/PlaceholderParticles/RobotSplat.RobotSplat" hitLocation))

(event EventDebugDespawnFX
  ;[1 1 1] Debug particle
  (bind _debugwindupfx (Variables|Default|GetDebugWindUpFX)
    (:then
      (Components|DestroyComponent _debugwindupfx))
    (:else)))

(event EventDebugSpawnFX
  (bind _lefthanddebugbox (Variables|Default|GetLeftHandDebugBox))
  (bind _righthanddebugbox (Variables|Default|GetRightHandDebugBox))
  (bind _leftfootdebugbox (Variables|Default|GetLeftFootDebugBox))
  (bind _rightfootdebugbox (Variables|Default|GetRightFootDebugBox))
  (bind _leftkneedebugbox (Variables|Default|GetLeftKneeDebugBox))
  (bind _rightkneedebugbox (Variables|Default|GetRightKneeDebugBox))
  (bind _array (Utilities|Array|MakeArray _lefthanddebugbox _righthanddebugbox _leftfootdebugbox _rightfootdebugbox _leftkneedebugbox _rightkneedebugbox))
  ;[1 1 1] Debug particle
  (bind _returnvalue (Effects|SpawnEmitterAttached "/Game/Effects/Particles/Fire/P_LargeFire.P_LargeFire" (Utilities|Select :Index (Variables|Default|GetcurrentAttackHitboxType) :Default 0 :HeldObject 0 :Projectile 0 :LeftHand (Utilities|Array|Get(acopy) _array) :LeftElbow 0 :LeftKnee (Utilities|Array|Get(acopy) _array 4) :LeftFoot (Utilities|Array|Get(acopy) _array 2) :RightHand (Utilities|Array|Get(acopy) _array 1) :RightElbow 0 :RightKnee (Utilities|Array|Get(acopy) _array 5) :RightFoot (Utilities|Array|Get(acopy) _array 3)) "None"))
  (Variables|Default|SetDebugWindUpFX _returnvalue))

(fn ConstructionScript)