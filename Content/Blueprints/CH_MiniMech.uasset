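; CH_MiniMech is the mini mech character, with its own attached sound, a spotlight and a fixed behavior value returned by GetBehavior.
; BeginPlay attaches a spatialized sound to the capsule and stores it for later.
; On defeat, if that sound is valid, it fades out while timelines drive its pitch and the spotlight intensity.
; When the light timeline finishes, the actor gets a delayed-destruction lifespan.
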(event EventBeginPlay
  (bind _returnvalue (Audio|SpawnSoundAttached "/Game/Sound/Audio/minimechsfx.minimechsfx" (Variables|Default|GetCapsuleComponent) "None" "0, 0, 0" "0, 0, 0" "KeepRelativeOffset" true 0.5 1.0 0.0 "/Game/Sound/InverseSoundAttenuation.InverseSoundAttenuation" 0 false))
  (Variables|Default|SetCurrentSound _returnvalue))

(event EventEventIsDefeated
  (bind _currentsound (Variables|Default|GetCurrentSound)
    (:then
      (Audio|Components|Audio|FadeOut _currentsound 5.0 0.0 "Linear" :!class /Script/Engine.AudioComponent)
      (Utilities|FlowControl|Sequence
        (:then_0
          (bind _pitch (Timeline|PitchEnd PlayFromStart)
            (:Update
              (Audio|Components|Audio|SetPitchMultiplier (Variables|Default|GetCurrentSound) _pitch))))
        (:then_1
          (bind _light (Timeline|LightEnd PlayFromStart)
            (:Update
              (Rendering|Components|Light|SetIntensity (Variables|Default|GetSpotLight) _light))
            (:Finished
              (Actor|SetLifeSpan 6e+01))))))
    (:else)))

(fn ConstructionScript)

(fn GetBehavior
  (return "NewEnumerator0"))