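; Special door interactable that opens once every object in its interaction list reports defeated, or stays open when the list is empty.
; A bound unlock-check event picks the open or closed offset, and Tick moves the door toward it at constant speed.
; Doors set to start opened are placed open at construction and close on first interaction.
; Activation can optionally print display text.
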(event Custom|CheckDoorUnlockRequirements_Event
  ;[1 1 1] Event for checking whether or not to open the door
  (if (> (Utilities|Array|Length (Variables|DoorSettings|GetListOfObjectsToInteractWith)) 0)
    (Variables|Default|SetbDoorShouldOpen true)
    (bind _array_element (Utilities|Array|ForEachLoopwithBreak (Variables|DoorSettings|GetListOfObjectsToInteractWith))
      (:LoopBody
        (bind _returnvalue (Class|CharacterInterface|GetIsDefeated _array_element))
        (if (not _returnvalue)
          (CallFunction|BreakLoopandCancelDoorOpen)
          (Variables|Default|SetbDoorShouldOpen false)))
      (:Completed
        (if (Variables|Default|GetbDoorShouldOpen)
          (Variables|Default|SetcurrentTargetLocation (Variables|DoorSettings|GetopenLocation))
          (if (Variables|DoorSettings|GetbSpawnTextOnActivate)
            (Development|PrintString (Variables|DoorSettings|GetSpawnDisplayText) true true "(R=0.000000,G=0.660000,B=1.000000,A=1.000000)" 3e+01)))))
    (else
      (Variables|Default|SetcurrentTargetLocation (Variables|DoorSettings|GetopenLocation)))))

(event Custom|BreakLoopAndCancelDoorOpen
  ;[1 1 1] Event for checking whether or not to open the door
  (Utilities|Array|ForEachLoopwithBreak (Variables|DoorSettings|GetListOfObjectsToInteractWith)) ; enters at Break
)

(event EventBeginPlay
  ;[1 1 1] Initialization
  (|CallParentFunction)
  (EventDispatchers|BindEventtoCheckDoorUnlockRequirements (delegate Custom|CheckDoorUnlockRequirements_Event))
  (if (> (Utilities|Array|Length (Variables|DoorSettings|GetListOfObjectsToInteractWith)) 0)
    (Variables|Default|SetcurrentTargetLocation (Variables|DoorSettings|GetclosedLocation))
    (else
      (Variables|Default|SetcurrentTargetLocation (Variables|DoorSettings|GetopenLocation))))
  (if (Variables|DoorSettings|GetStartOpened)
    (Variables|Default|SetcurrentTargetLocation (Variables|DoorSettings|GetopenLocation))))

(event Collision|EventActorBeginOverlap
  (params (OtherActor :type Actor%20Object%20Reference))
  (|CallParentFunction OtherActor) ; This node is disabled and will not be called.\nDrag off pins to build functionality.
)

(event EventTick
  (params (DeltaSeconds :type Float%20%28single-precision%29))
  ;[1 1 1] DoorLocationSet
  (|CallParentFunction DeltaSeconds)
  (Transformation|SetWorldLocation (Variables|Default|GetDoorObject) (Math|Interpolation|VInterptoConstant (Transformation|GetWorldLocation (Variables|Default|GetDoorObject)) (+ (Variables|Default|GetinitialLocation) (Variables|Default|GetcurrentTargetLocation)) DeltaSeconds (Variables|DoorSettings|GetDoorSpeed)) false false))

(event EventObjectInteracted
  (params (InteractorActor :type Actor%20Object%20Reference))
  ;[1 1 1] For StartOpened
  (Utilities|FlowControl|Sequence
    (:then_0
      (if (Variables|DoorSettings|GetbSpawnTextOnActivate)
        (Development|PrintString (Variables|DoorSettings|GetSpawnDisplayText) true true "(R=0.000000,G=0.660000,B=1.000000,A=1.000000)" 3e+01)))
    (:then_1
      (Utilities|FlowControl|DoOnce false
        (:Completed
          (if (Variables|DoorSettings|GetStartOpened)
            (Variables|Default|SetcurrentTargetLocation (Variables|DoorSettings|GetclosedLocation))))))))

(fn ConstructionScript
  (|CallParentFunction)
  (Variables|Default|SetinitialLocation (Transformation|GetWorldLocation (Variables|Default|GetDoorObject)))
  (if (Variables|DoorSettings|GetStartOpened)
    (bind _output_get (Variables|Default|SetcurrentTargetLocation (Variables|DoorSettings|GetopenLocation)))
    (Transformation|SetWorldLocation (Variables|Default|GetDoorObject) (+ (Transformation|GetWorldLocation (Variables|Default|GetDoorObject)) _output_get) false false)
    (else
      (bind _output_get_2 (Variables|Default|SetcurrentTargetLocation (Variables|DoorSettings|GetclosedLocation)))
      (Transformation|SetWorldLocation (Variables|Default|GetDoorObject) (+ _output_get_2 (Transformation|GetWorldLocation (Variables|Default|GetDoorObject))) false false))))