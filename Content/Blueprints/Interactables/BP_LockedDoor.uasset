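; Locked door that slides open once every enemy in its assigned list is defeated, or from the start if the list is empty.
; A bound CheckDoorUnlockRequirements event checks each enemy's defeated state and sets the target offset to open or closed.
; Tick moves the door mesh at constant speed toward its initial location plus that offset using VInterpToConstant.
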(event Custom|CheckDoorUnlockRequirements_Event
  ;[1 1 1] Event for checking whether or not to open the door
  (if (> (Utilities|Array|Length (Variables|Default|GetListOfEnemiesToDefeat)) 0)
    (Variables|Default|SetbDoorShouldOpen true)
    (bind _array_element (Utilities|Array|ForEachLoopwithBreak (Variables|Default|GetListOfEnemiesToDefeat))
      (:LoopBody
        (bind _returnvalue (Class|CharacterInterface|GetIsDefeated _array_element))
        (if (not _returnvalue)
          (CallFunction|BreakLoopandCancelDoorOpen)
          (Variables|Default|SetbDoorShouldOpen false)))
      (:Completed
        (if (Variables|Default|GetbDoorShouldOpen)
          (Variables|Default|SetcurrentTargetLocation (Variables|Default|GetopenLocation))
          (else
            (Variables|Default|SetcurrentTargetLocation (Variables|Default|GetclosedLocation))))))
    (else
      (Variables|Default|SetcurrentTargetLocation (Variables|Default|GetopenLocation)))))

(event Custom|BreakLoopAndCancelDoorOpen
  ;[1 1 1] Event for checking whether or not to open the door
  (Utilities|Array|ForEachLoopwithBreak (Variables|Default|GetListOfEnemiesToDefeat)) ; enters at Break
)

(event EventBeginPlay
  ;[1 1 1] Initialization
  (Variables|Default|SetinitialLocation (Transformation|GetWorldLocation (Variables|Default|GetDoorObject)))
  (|CallParentFunction)
  (EventDispatchers|BindEventtoCheckDoorUnlockRequirements (delegate Custom|CheckDoorUnlockRequirements_Event))
  (if (> (Utilities|Array|Length (Variables|Default|GetListOfEnemiesToDefeat)) 0)
    (Variables|Default|SetcurrentTargetLocation (Variables|Default|GetclosedLocation))
    (else
      (Variables|Default|SetcurrentTargetLocation (Variables|Default|GetopenLocation)))))

(event Collision|EventActorBeginOverlap
  (params (OtherActor :type Actor%20Object%20Reference))
  (|CallParentFunction OtherActor) ; This node is disabled and will not be called.\nDrag off pins to build functionality.
)

(event EventTick
  (params (DeltaSeconds :type Float%20%28single-precision%29))
  ;[1 1 1] DoorLocationSet
  (|CallParentFunction DeltaSeconds)
  (Transformation|SetWorldLocation (Variables|Default|GetDoorObject) (Math|Interpolation|VInterptoConstant (Transformation|GetWorldLocation (Variables|Default|GetDoorObject)) (+ (Variables|Default|GetinitialLocation) (Variables|Default|GetcurrentTargetLocation)) DeltaSeconds (Variables|Default|GetDoorSpeed)) false false))

(fn ConstructionScript
  (|CallParentFunction))