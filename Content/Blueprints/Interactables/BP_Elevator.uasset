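; An interactable elevator actor that travels between its placed position and an end offset, switching destination each time it is interacted with.
; The construction script records the starting location, and ObjectInteracted flips GoingUp to set the target offset to either EndLocation or zero.
; Tick continuously moves the actor toward that target at constant ElevatorSpeed using VInterpToConstant, without sweeping for collisions.
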(event EventBeginPlay
  (|CallParentFunction) ; This node is disabled and will not be called.\nDrag off pins to build functionality.
)

(event Collision|EventActorBeginOverlap
  (params (OtherActor :type Actor%20Object%20Reference))
  (|CallParentFunction OtherActor) ; This node is disabled and will not be called.\nDrag off pins to build functionality.
)

(event EventTick
  (params (DeltaSeconds :type Float%20%28single-precision%29))
  ;[1 1 1] Tick
  (|CallParentFunction DeltaSeconds)
  (Transformation|SetActorLocation (Math|Interpolation|VInterptoConstant (Transformation|GetActorLocation) (+ (Variables|Default|GetInitialLocation) (Variables|Default|GetTargetLocation)) DeltaSeconds (Variables|ElevatorSettings|GetElevatorSpeed)) false false))

(event EventObjectInteracted
  (params (InteractorActor :type Actor%20Object%20Reference))
  ;[1 1 1] Interact procedure
  (if (Variables|Default|GetbGoingUp)
    (Variables|Default|SetbGoingUp false)
    (Variables|Default|SetTargetLocation (Variables|ElevatorSettings|GetEndLocation))
    (else
      (Variables|Default|SetbGoingUp true)
      (Variables|Default|SetTargetLocation "0, 0, 0"))))

(fn ConstructionScript
  (|CallParentFunction)
  (Variables|Default|SetInitialLocation (Transformation|GetActorLocation)))