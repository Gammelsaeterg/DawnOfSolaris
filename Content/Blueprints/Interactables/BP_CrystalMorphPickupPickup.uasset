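; BP_CrystalMorphPickupPickup is an interactable crystal pickup that unlocks a combat moveset for the actor interacting with it.
; On interaction it sends the unlock message with its CombatMovesetIndex and hides the Crystal component rather than destroying the actor.
; For an alien player character, it then remaps the index through a Select to update crystal materials and initializes the crystal colors.
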(event EventBeginPlay
  (|CallParentFunction) ; This node is disabled and will not be called.\nDrag off pins to build functionality.
)

(event Collision|EventActorBeginOverlap
  (params (OtherActor :type Actor%20Object%20Reference))
  (|CallParentFunction OtherActor) ; This node is disabled and will not be called.\nDrag off pins to build functionality.
)

(event EventTick
  (params (DeltaSeconds :type Float%20%28single-precision%29))
  (|CallParentFunction DeltaSeconds) ; This node is disabled and will not be called.\nDrag off pins to build functionality.
)

(event EventObjectInteracted
  (params (InteractorActor :type Actor%20Object%20Reference))
  (Class|CharacterInterface|UnlockMoveset(Message) InteractorActor (Variables|InteractionObjectSettings|GetCombatMovesetIndex))
  (Rendering|SetVisibility (Variables|Default|GetCrystal) false false)
  (bind _asch_alien_player_character (Utilities|Casting|CastToCH_AlienPlayerCharacter InteractorActor))
  (Default|UpdateCrystalMaterials _asch_alien_player_character (Utilities|Select :Index (Variables|InteractionObjectSettings|GetCombatMovesetIndex) :Option%200 0 :Option%201 2 :Option%202 1))
  (Default|InitializeCrystalColors _asch_alien_player_character))

(fn ConstructionScript
  (|CallParentFunction))