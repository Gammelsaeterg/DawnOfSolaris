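; A trigger box that starts the end cutscene when an alien player character overlaps it.
; The first successful overlap finds that player's controller through its player ID and calls PlayVideo on its player UI.
; It then tells every ambient audio and level music actor to fade out.
; An unconnected timeline that would lower the game instance's music and sound volumes is left in the graph and never runs.
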(event EventBeginPlay)

(event Collision|EventActorBeginOverlap
  (params (OtherActor :type Actor%20Object%20Reference))
  (bind _asch_alien_player_character (Utilities|Casting|CastToCH_AlienPlayerCharacter OtherActor))
  (bind _asbp_default_player_controller (Utilities|Casting|CastToBP_DefaultPlayerController (Game|GetPlayerController (Variables|/Script/DawnOfSolaris.BaseCharacter|GetcurrentPlayerID _asch_alien_player_character))))
  (bind _asui_player_ui (Utilities|Casting|CastToUI_PlayerUI (Variables|/Script/DawnOfSolaris.DefaultPlayerController|GetPlayerUI _asbp_default_player_controller)))
  (Utilities|FlowControl|DoOnce false
    (:Completed
      (Default|PlayVideo _asui_player_ui)
      (bind _outactors (Actor|GetAllActorsOfClass "/Game/Blueprints/BP_AmbientAudio.BP_AmbientAudio_C"))
      (for _array_element _outactors
        (Default|FadeOutAudio _array_element))
      (bind _outactors_2 (Actor|GetAllActorsOfClass "/Game/Blueprints/BP_LevelMusic.BP_LevelMusic_C"))
      (for _array_element_2 _outactors_2
        (Default|FadeOutAudio _array_element_2)))))

(event EventTick
  (params (DeltaSeconds :type Float%20%28single-precision%29)))

(fn ConstructionScript)