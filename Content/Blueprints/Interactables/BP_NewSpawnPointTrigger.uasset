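; BP_NewSpawnPointTrigger is an interactable that sets a new respawn point for the alien player.
; On ObjectInteracted, it casts the interactor to CH_AlienPlayerCharacter and stores that character's current location, rather than the trigger's own, as its RespawnLocation.
; Despite the name, it has no active overlap logic, and its debug print is disconnected.
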(event EventBeginPlay
  (|CallParentFunction) ; This node is disabled and will not be called.\nDrag off pins to build functionality.
)

(event Collision|EventActorBeginOverlap
  (params (OtherActor :type Actor%20Object%20Reference))
  (|CallParentFunction OtherActor) ; This node is disabled and will not be called.\nDrag off pins to build functionality.
)

(event EventTick
  (params (DeltaSeconds :type Float%20%28single-precision%29))
  (|CallParentFunction DeltaSeconds) ; This node is disabled and will not be called.\nDrag off pins to build functionality.
)

(event EventObjectInteracted
  (params (InteractorActor :type Actor%20Object%20Reference))
  (bind _asch_alien_player_character (Utilities|Casting|CastToCH_AlienPlayerCharacter InteractorActor))
  (Variables|/Game/Blueprints/CH_AlienPlayerCharacter.CH_AlienPlayerCharacter_C|SetRespawnLocation _asch_alien_player_character (Transformation|GetActorLocation _asch_alien_player_character)))

(fn ConstructionScript
  (|CallParentFunction))