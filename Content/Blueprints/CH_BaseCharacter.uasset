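; Base character Blueprint that tracks its owning player and exposes a behavior state.
; On possession by a PlayerController it stores that controller's ID as the current player index.
; A getter returns the current behavior tree enum, and an unconnected debug block would print the launched state.
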(event EventTick
  (params (DeltaSeconds :type Float%20%28single-precision%29))
  ;[1 1 1] Debug prints, TODO: Delete/disable when not needed
)

(event EventPossessed
  (params (NewController :type Controller%20Object%20Reference))
  ;[1 1 1] SetPlayerIndex
  (bind _asplayer_controller (Utilities|Casting|CastToPlayerController NewController))
  (Variables|Default|SetcurrentPlayerID (Class|GameplayStatics|GetPlayerControllerID _asplayer_controller)))

(fn ConstructionScript)

(fn GetBehavior
  (return (Variables|Default|GetcurrentBTEnum)))