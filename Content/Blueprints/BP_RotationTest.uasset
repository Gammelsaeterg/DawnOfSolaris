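; BP_RotationTest is a pawn Blueprint, apparently for testing, that moves along world axes from hard-coded WASD key events.
; W/S and D/A set two axis values to positive or negative one on press and reset them to zero on release.
; Tick feeds both values into AddMovementInput as world X and Y direction.
; Despite the name, the graphs contain no rotation logic.
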(event EventBeginPlay)

(event Collision|EventActorBeginOverlap
  (params (OtherActor :type Actor%20Object%20Reference)))

(event EventTick
  (params (DeltaSeconds :type Float%20%28single-precision%29))
  (Pawn|Input|AddMovementInput (Math|Vector|MakeVector (Variables|Default|Get0_0) (Variables|Default|Get0_2) 0.0) 1.0 false))

(event Input|KeyboardEvents|W
  (params (Key :type Key%20Structure :default "None"))
  (:Pressed
    (Variables|Default|Set0_0 1.0))
  (:Released
    (Variables|Default|Set0_0 0.0)))

(event Input|KeyboardEvents|S
  (params (Key :type Key%20Structure :default "None"))
  (:Pressed
    (Variables|Default|Set0_0 -1.0))
  (:Released
    (Variables|Default|Set0_0 0.0)))

(event Input|KeyboardEvents|A
  (params (Key :type Key%20Structure :default "None"))
  (:Pressed
    (Variables|Default|Set0_2 -1.0))
  (:Released
    (Variables|Default|Set0_2 0.0)))

(event Input|KeyboardEvents|D
  (params (Key :type Key%20Structure :default "None"))
  (:Pressed
    (Variables|Default|Set0_2 1.0))
  (:Released
    (Variables|Default|Set0_2 0.0)))

(fn ConstructionScript)