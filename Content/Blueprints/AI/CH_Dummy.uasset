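; CH_Dummy is an AI dummy character blueprint that exposes Attack and Hook events, each taking a target actor.
; Attack yaws the actor toward a valid target, then calls StartDefaultAttack.
; Hook spawns BP_Claw at the Claw component's world transform, adjusting for collisions, after setting yaw from a look-at of its own location to itself, so it ignores the target's position.
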(event Custom|Hook
  (params (TargetActor :type Actor%20Object%20Reference))
  (bind _claw (Variables|Default|GetClaw))
  (Utilities|FlowControl|Sequence
    (:then_0
      (Utilities|IsValid TargetActor
        (:Is%20Valid
          (Transformation|SetActorRotation (Math|Rotator|MakeRotator 0.0 0.0 (.yaw (Math|Rotator|FindLookatRotation (Transformation|GetActorLocation) (Transformation|GetActorLocation))))))))
    (:then_1
      (Game|SpawnActorfromClass "/Game/Blueprints/AI/Abilities/BP_Claw.BP_Claw_C" (Math|Transform|MakeTransform (Transformation|GetWorldLocation _claw) (Transformation|GetWorldRotation _claw)) "AdjustIfPossibleButDontSpawnIfColliding" 0 0))))

(event Custom|Attack
  (params (Target%20Actor :type Actor%20Object%20Reference))
  (Utilities|FlowControl|Sequence
    (:then_0
      (Utilities|IsValid Target%20Actor
        (:Is%20Valid
          (Transformation|SetActorRotation (Math|Rotator|MakeRotator 0.0 0.0 (.yaw (Math|Rotator|FindLookatRotation (Transformation|GetActorLocation) (Transformation|GetActorLocation Target%20Actor))))))))
    (:then_1
      (Class|CharacterInterface|StartDefaultAttack))))

(fn ConstructionScript)