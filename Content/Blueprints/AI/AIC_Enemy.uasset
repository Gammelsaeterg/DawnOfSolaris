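; AI controller for enemy pawns that picks a melee, ranged or commander behavior tree on possess, based on the pawn's behavior message.
; AI perception updates on player-aligned actors write line-of-sight, target and abort-combat Blackboard keys through small helper functions.
; Losing sight flags combat to abort at once but clears the target only after a delay timer, which is cancelled if the player is sensed again.
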(event OnTargetPerceptionUpdated(AIPerception)
  (params (Actor :type Actor%20Object%20Reference) (Stimulus :type AI%20Stimulus%20Structure))
  ;[1 1 1] When the AI perceives something, store Actor as a variable to later update the bb
  (bind _output_get (Variables|Default|SetPerceived%20Actor Actor))
  (bind _returnvalue (Class|CharacterInterface|GetAlignment(Message) _output_get))
  (if (Utilities|Enum|Equal(Enum) _returnvalue "Player")
    (if (.bSuccessfullySensed (Utilities|Struct|BreakAIStimulus Stimulus))
      (Utilities|Time|ClearandInvalidateTimerbyHandle (Variables|Default|GetLostSightTimer))
      (CallFunction|UpdateSightKey true)
      (CallFunction|UpdateTargetKey (Variables|Default|GetPerceived%20Actor))
      (CallFunction|UpdateCombatKey false)
      (else
        (bind _returnvalue_2 (Utilities|Time|SetTimerbyEvent (delegate Custom|LostSight) 15.0))
        (Variables|Default|SetLostSightTimer _returnvalue_2)
        (CallFunction|UpdateSightKey false)
        (CallFunction|UpdateCombatKey true)))))

(event Custom|LostSight
  (CallFunction|UpdateTargetKey))

(event EventBeginPlay)

(event EventTick
  (params (DeltaSeconds :type Float%20%28single-precision%29)))

(event EventPossess
  (params (PossessedPawn :type Pawn%20Object%20Reference))
  (bind _outbehavior (Class|InterfaceAI|GetBehavior(Message) PossessedPawn))
  (switch Utilities|FlowControl|Switch|SwitchonENonPlayerCharacterBehavior _outbehavior
    (:NewEnumerator0
      (AI|RunBehaviorTree "/Game/Blueprints/AI/BT_GruntMelee.BT_GruntMelee"))
    (:NewEnumerator1
      (AI|RunBehaviorTree "/Game/Blueprints/AI/BT_GruntRanged.BT_GruntRanged"))
    (:NewEnumerator2
      (AI|RunBehaviorTree "/Game/Blueprints/AI/BT_Commander.BT_Commander"))))

(fn ConstructionScript)

(fn UpdateSightKey
  (params (HasLineOfSight :type Boolean))
  ;[1 1 1] Updates the HasLineOfSight BB key
  (AI|Components|Blackboard|SetValueasBool (Variables|Default|GetBlackboard) (Utilities|Name|MakeLiteralName "HasLineOfSight") HasLineOfSight))

(fn UpdateTargetKey
  (params (TargetActor :type Actor%20Object%20Reference))
  ;[1 1 1] Updates the TargetActor BB key with actor passed through
  (AI|Components|Blackboard|SetValueasObject (Variables|Default|GetBlackboard) (Utilities|Name|MakeLiteralName "TargetActor") TargetActor))

(fn UpdateCombatKey
  (params (Abort%20Combat :type Boolean))
  (AI|Components|Blackboard|SetValueasBool (Variables|Default|GetBlackboard) (Utilities|Name|MakeLiteralName "AbortCombat") Abort%20Combat)
  (Development|PrintString (Utilities|String|ToString(Boolean) Abort%20Combat)))