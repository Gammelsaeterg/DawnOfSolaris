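; Gatling gun ability that fires a stream of projectiles in timed bursts once engaged.
; Engage uses a DoOnce to start a looping timer at FireRate, plus an eight-second timer that calls Disengage to stop firing and re-arm it.
; Each tick of the looping timer spawns a BP_GatlingProjectile at the socket the weapon mesh is attached to.
; Muzzle effect and older FireProjectile nodes are left unwired.
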(event Custom|Engage
  (Variables|Default|SetEngaging true)
  (if (Variables|Default|GetEngaging)
    (Utilities|FlowControl|DoOnce false :!label _label
      (:Completed
        (bind _returnvalue (Utilities|Time|SetTimerbyEvent (delegate Custom|PrepareFiring) (Variables|Default|GetFireRate) true))
        (Variables|Default|SetFireTimer _returnvalue)
        (Utilities|Time|SetTimerbyEvent (delegate Custom|Disengage) 8.0)))
    (else
      (Utilities|Time|ClearandInvalidateTimerbyHandle (Variables|Default|GetFireTimer))
      (goto _label Reset))))

(event Custom|Disengage
  (Variables|Default|SetEngaging false)
  (if (Variables|Default|GetEngaging)
    (Utilities|FlowControl|DoOnce false :!label _label
      (:Completed
        (bind _returnvalue (Utilities|Time|SetTimerbyEvent (delegate Custom|PrepareFiring) (Variables|Default|GetFireRate) true))
        (Variables|Default|SetFireTimer _returnvalue)
        (Utilities|Time|SetTimerbyEvent (delegate Custom|Disengage) 8.0)))
    (else
      (Utilities|Time|ClearandInvalidateTimerbyHandle (Variables|Default|GetFireTimer))
      (goto _label Reset))))

(event Custom|PrepareFiring
  (CallFunction|Fire))

(event EventBeginPlay)

(event Collision|EventActorBeginOverlap
  (params (OtherActor :type Actor%20Object%20Reference)))

(event EventTick
  (params (DeltaSeconds :type Float%20%28single-precision%29)))

(fn ConstructionScript)

(fn Fire
  (bind _weaponmesh (Variables|Default|GetWeaponMesh))
  (Game|SpawnActorfromClass "/Game/Blueprints/Weapons/BP_GatlingProjectile.BP_GatlingProjectile_C" (Transformation|GetSocketTransform (Transformation|GetAttachParent _weaponmesh) (Transformation|GetAttachSocketName _weaponmesh) "RTS_World") "Undefined" 0 0))