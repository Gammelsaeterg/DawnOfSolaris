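; BP_Missile is a homing missile projectile that chases player 0 and explodes with radial damage, sound and effects.
; Tick runs Guidance, which after a short Delay turns the missile toward the player at constant speed and resets velocity along its forward vector.
; A projectile bounce spawns a fading decal and impact emitter before exploding, while a timer self-destructs it otherwise.
; An arced midpoint is calculated before Target is set but goes unused here.
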(event OnProjectileBounce(ProjectileMovement)
  (params (ImpactResult :type Hit%20Result%20Structure%20%28by%20ref%29) (ImpactVelocity :type Vector%20%28by%20ref%29 :default "0, 0, 0"))
  (bind (_bblockinghit _binitialoverlap _time _distance _location _impactpoint _normal _impactnormal) (Collision|BreakHitResult ImpactResult))
  (bind _self self)
  (bind _returnvalue (Transformation|GetActorTransform _self))
  (bind (_location_2 _rotation) (Math|Transform|BreakTransform _returnvalue))
  (CallFunction|SpawnImpact _location (Math|Conversions|RotationFromXVector _impactnormal))
  ;[1 1 1] Apply damage in a radius
  (Game|Damage|ApplyRadialDamage (Variables|Default|GetDamage) _location_2 (Variables|Default|GetDamageRadius) 0 0 0 0 false "ECC_Visibility")
  ;[1 1 1] Explosion sound
  (Audio|SpawnSoundatLocation "/Game/Audio/explosion2.explosion2" _location_2 "0, 0, 0" 1.0 1.0 0.0 0 0)
  ;[1 1 1] Destroy after impact
  (Actor|DestroyActor self))

(event Custom|Self%20Destruct
  (bind _self self)
  (bind _returnvalue (Transformation|GetActorTransform _self))
  (bind (_location _rotation) (Math|Transform|BreakTransform _returnvalue))
  (Effects|SpawnEmitteratLocation "/Game/Effects/Particles/Explosions/p_explosion.p_explosion" _location _rotation "0.100000,0.100000,0.100000")
  ;[1 1 1] Apply damage in a radius
  (Game|Damage|ApplyRadialDamage (Variables|Default|GetDamage) _location (Variables|Default|GetDamageRadius) 0 0 0 0 false "ECC_Visibility")
  ;[1 1 1] Explosion sound
  (Audio|SpawnSoundatLocation "/Game/Audio/explosion2.explosion2" _location "0, 0, 0" 1.0 1.0 0.0 0 0)
  ;[1 1 1] Destroy after impact
  (Actor|DestroyActor self))

(event Custom|Guidance
  (params (DeltaT :type Float%20%28single-precision%29))
  (bind _sphere (Variables|Default|GetSphere))
  (bind _returnvalue (Transformation|GetWorldRotation _sphere))
  ;[0.2384 0.4922 1] Missile guidance event
  (Variables|Default|SetDeltaT DeltaT)
  ;;[1 1 1] Small delay to offset the players position
  (Utilities|FlowControl|Delay 0.3)
  (Transformation|SetActorRotation (Class|KismetMathLibrary|RInterptoConstant _returnvalue (Math|Rotator|FindLookatRotation (Transformation|GetActorLocation self) (Transformation|GetActorLocation (Variables|Default|GetTarget))) (Variables|Default|GetDeltaT) (Variables|Default|GetRotation)))
  (Variables|/Script/Engine.MovementComponent|SetVelocity (Variables|Default|GetProjectileMovement) (* (Math|Vector|GetForwardVector _returnvalue) (Variables|Default|GetMissileSpeed)))
  (Development|PrintString (Utilities|GetDisplayName (Variables|Default|GetTarget))))

(event EventTick
  (params (DeltaSeconds :type Float%20%28single-precision%29))
  (CallFunction|Guidance DeltaSeconds))

(event EventBeginPlay
  (CallFunction|CalculateInitialTravel)
  (Variables|Default|SetTarget (Game|GetPlayerCharacter 0))
  (Utilities|Time|SetTimerbyEvent (delegate Custom|Self%20Destruct) 5.0))

(fn ConstructionScript)

(fn SpawnImpact
  (params (Location :type Vector) (Rotation :type Rotator))
  ;[1 1 1] Function to spawn impact decal and impact particle effect (explosion)
  (bind _returnvalue (Rendering|Decal|SpawnDecalatLocation (Variables|Default|GetImpact%20decal) "50.000000,250.000000,250.000000" Location Rotation 0.0))
  (Rendering|Components|Decal|SetFadeOut _returnvalue 5.0 2.0 true)
  (Rendering|Components|Decal|SetFadeScreenSize _returnvalue 0.0001)
  (Effects|SpawnEmitteratLocation (Variables|Default|GetImpact%20emitter) Location Rotation "0.100000,0.100000,0.100000"))

(fn CalculateInitialTravel
  (bind _self self)
  (bind _target (Variables|Default|GetTarget))
  (bind _returnvalue (Transformation|GetActorLocation _self))
  (bind _returnvalue_2 (Transformation|GetActorLocation _target))
  (bind _returnvalue_3 (+ _returnvalue _returnvalue_2))
  (bind _returnvalue_4 (/ _returnvalue_3 2))
  (bind (_x _y _z) (Math|Vector|BreakVector _returnvalue_4))
  (Variables|Default|SetInitial%20Travel%20Location (Math|Vector|MakeVector _x _y (+ _z 5e+02))))