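; AI missile launcher ability that targets the player pawn on begin play and spawns BP_Missile with muzzle flash and sound.
; Engage starts a looping timer that cycles through right and left tube ports, then auto-disengages after a fixed delay, clearing the timer.
; The timer's Fire function is an empty stub with disconnected spawn logic.
; Actual spawning happens in FireFromMontage at a supplied transform, apparently for animation montages to call.
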(event Custom|Set%20Target
  (Variables|Default|SetCurrentTarget (Game|Player|GetPlayerPawn 0)))

(event Custom|Engage
  (Variables|Default|SetEngaging true)
  (if (Variables|Default|GetEngaging)
    (Utilities|FlowControl|DoOnce false :!label _label
      (:Completed
        ;[1 1 1] Start firing event with timer
        (bind _returnvalue (Utilities|Time|SetTimerbyEvent (delegate Custom|PrepareLaunch) (Variables|Default|GetFire%20rate) true))
        (Variables|Default|SetFire%20Timer _returnvalue)
        (Utilities|Time|SetTimerbyEvent (delegate Custom|Disengage) 6.0)))
    (else
      (Utilities|Time|ClearandInvalidateTimerbyHandle (Variables|Default|GetFire%20Timer))
      (goto _label Reset))))

(event Custom|Disengage
  (Variables|Default|SetEngaging false)
  (if (Variables|Default|GetEngaging)
    (Utilities|FlowControl|DoOnce false :!label _label
      (:Completed
        ;[1 1 1] Start firing event with timer
        (bind _returnvalue (Utilities|Time|SetTimerbyEvent (delegate Custom|PrepareLaunch) (Variables|Default|GetFire%20rate) true))
        (Variables|Default|SetFire%20Timer _returnvalue)
        (Utilities|Time|SetTimerbyEvent (delegate Custom|Disengage) 6.0)))
    (else
      (Utilities|Time|ClearandInvalidateTimerbyHandle (Variables|Default|GetFire%20Timer))
      (goto _label Reset))))

(event Custom|PrepareLaunch
  ;[1 1 1] If current port is last, switch back to the first
  (if (== (Variables|Default|GetCurrent%20Launch%20Port) (Utilities|Array|Length (Variables|Default|GetLaunch%20Port%20Array)))
    (Variables|Default|SetCurrent%20Launch%20Port 0))
  ;[1 1 1] Fire and increment launch port
  (CallFunction|Fire (Utilities|Array|Get(acopy) (Variables|Default|GetLaunch%20Port%20Array) (Variables|Default|GetCurrent%20Launch%20Port)))
  (Math|Integer|IncrementInt (Variables|Default|GetCurrent%20Launch%20Port)
    (:%20%20
      (Development|PrintString "Firing Missiles"))))

(event EventBeginPlay
  ;[1 1 1] Set initial values and load launch port array
  (Utilities|FlowControl|Sequence
    (:then_0
      (CallFunction|LoadPortArray)
      (CallFunction|SetTarget))))

(fn ConstructionScript)

(fn Fire
  (params (LaunchPort :type Arrow%20Component%20Object%20Reference)))

(fn LoadPortArray
  (bind _launch_port_array (Variables|Default|GetLaunch%20Port%20Array))
  (Utilities|Array|Add _launch_port_array (Variables|Default|GetTubeR))
  (Utilities|Array|Add _launch_port_array (Variables|Default|GetTubeL)))

(fn FirefromMontage
  (params (FireTransform :type Transform))
  (bind (_location _rotation _scale) (Math|Transform|BreakTransform FireTransform))
  ;[1 1 1] Spawn launch particle at port
  (Effects|SpawnEmitteratLocation "/Game/Particles/PlaceholderParticles/MuzzleFlash.MuzzleFlash" _location _rotation _scale false)
  ;[1 1 1] Spawn missile and sound effect
  (Game|SpawnActorfromClass "/Game/Blueprints/AI/Abilities/MissileLauncher/BP_Missile.BP_Missile_C" FireTransform "Undefined" 0 0)
  (Audio|PlaySoundatLocation 0 _location "0, 0, 0" 1.0 1.0 0.0 0 0 0))