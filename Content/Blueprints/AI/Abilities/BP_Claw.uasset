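; BP_Claw is a hook projectile in the AI abilities that drags tagged actors back to where it spawned.
; BeginPlay stores the collider's location, then after a short delay a timeline stops movement, lerps the claw back and destroys it.
; On hit, gameplay tags read through the OverlapInfo interface are queried; a match retracts the claw immediately while a second timeline pulls the hit actor to the origin.
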(event OnComponentHit(Collider)
  (params (HitComponent :type Primitive%20Component%20Object%20Reference) (OtherActor :type Actor%20Object%20Reference) (OtherComp :type Primitive%20Component%20Object%20Reference) (NormalImpulse :type Vector :default "0, 0, 0") (Hit :type Hit%20Result%20Structure%20%28by%20ref%29))
  ;[1 1 1] Interface to get gameplay tags of Other Actor
  (bind _tagcont (CallFunction|OverlapInfo OtherActor))
  (if (GameplayTags|DoesContainerMatchTagQuery _tagcont (GameplayTags|MakeGameplayTagQuery "(TokenStreamVersion=0,TagDictionary=((TagName=\"Explosive\"),(TagName=\"Player\")),QueryTokenStream=(0,1,1,2,0,1),UserDescription=\"\",AutoDescription=\" ANY( Explosive, Player )\")"))
    (Development|PrintString "Match")
    (Utilities|FlowControl|Sequence
      (:then_0
        (bind _newtrack_0 (Timeline|Timeline Play)
          (:Update
            (Variables|/Script/Engine.MovementComponent|SetVelocity (Variables|Default|GetProjectileMovement) "0, 0, 0")
            (Transformation|SetWorldLocation (Variables|Default|GetCollider) (Math|Vector|Lerp(Vector) (Transformation|GetWorldLocation (Variables|Default|GetCollider)) (stale EventBeginPlay _output_get) _newtrack_0) false false))
          (:Finished
            (Actor|DestroyActor))))
      (:then_1
        (bind _newtrack_0_2 (Timeline|Timeline_0 Play)
          (:Update
            (Transformation|SetWorldLocation (Variables|/Script/Engine.Actor|GetRootComponent OtherActor) (Math|Vector|Lerp(Vector) (Transformation|GetActorLocation OtherActor) (Variables|Default|GetLocation) _newtrack_0_2) false false))
          (:Finished
            (Actor|DestroyActor)))))
    (else
      (Development|PrintString "No match"))))

(event EventBeginPlay
  (bind _collider (Variables|Default|GetCollider))
  (bind _returnvalue (Transformation|GetWorldLocation _collider))
  ;[1 1 1] Initial location
  (bind _output_get (Variables|Default|SetLocation _returnvalue))
  (Utilities|FlowControl|Delay 1.0)
  (bind _newtrack_0 (Timeline|Timeline Play)
    (:Update
      (Variables|/Script/Engine.MovementComponent|SetVelocity (Variables|Default|GetProjectileMovement) "0, 0, 0")
      (Transformation|SetWorldLocation (Variables|Default|GetCollider) (Math|Vector|Lerp(Vector) _returnvalue _output_get _newtrack_0) false false))
    (:Finished
      (Actor|DestroyActor))))

(fn ConstructionScript)

(fn OverlapInfo
  (params (Target :type Actor%20Object%20Reference))
  (return 0 "(GameplayTags=((TagName=\"Player\"),(TagName=\"Explosive\")))"))