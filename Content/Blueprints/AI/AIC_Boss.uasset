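; AI controller for the boss that turns perception of Player-aligned actors into Blackboard state.
; The first perception update starts the BT_Slayer behavior tree through a DoOnce; Possess is empty.
; Sensing the player sets TargetActor and HasLineOfSight and cancels the sight timer.
; Losing the player clears HasLineOfSight at once, then a delayed LostSight timer clears TargetActor, giving a grace period.
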(event OnTargetPerceptionUpdated(AIPerception)
  (params (Actor :type Actor%20Object%20Reference) (Stimulus :type AI%20Stimulus%20Structure))
  (Utilities|FlowControl|Sequence
    (:then_0
      (Utilities|FlowControl|DoOnce false
        (:Completed
          (AI|RunBehaviorTree "/Game/Blueprints/AI/BT_Slayer.BT_Slayer"))))
    (:then_1
      (bind _output_get (Variables|Default|SetPerceived%20Actor Actor))
      (bind _returnvalue (Class|CharacterInterface|GetAlignment(Message) _output_get))
      (if (Utilities|Enum|Equal(Enum) _returnvalue "Player")
        (if (.bSuccessfullySensed (Utilities|Struct|BreakAIStimulus Stimulus))
          (Utilities|Time|ClearandInvalidateTimerbyHandle (Variables|Default|GetSight%20Timer))
          (CallFunction|UpdateSightKey true)
          (CallFunction|UpdateTargetKey (Variables|Default|GetPerceived%20Actor))
          (else
            (bind _returnvalue_2 (Utilities|Time|SetTimerbyEvent (delegate Custom|LostSight) 3e+01))
            (Variables|Default|SetSight%20Timer _returnvalue_2)
            (CallFunction|UpdateSightKey false)))))))

(event Custom|LostSight
  ;[1 1 1] Should boss ever lose sight?
  (CallFunction|UpdateTargetKey))

(event EventPossess
  (params (PossessedPawn :type Pawn%20Object%20Reference)))

(fn ConstructionScript)

(fn UpdateTargetKey
  (params (Target%20Actor :type Actor%20Object%20Reference))
  (AI|Components|Blackboard|SetValueasObject (Variables|Default|GetBlackboard) (Utilities|Name|MakeLiteralName "TargetActor") Target%20Actor))

(fn UpdateSightKey
  (params (HasLineOfSight :type Boolean))
  (AI|Components|Blackboard|SetValueasBool (Variables|Default|GetBlackboard) (Utilities|Name|MakeLiteralName "HasLineOfSight") HasLineOfSight))