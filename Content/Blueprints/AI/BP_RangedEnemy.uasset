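; Ranged enemy AI character that carries a gun and can shoot or take cover.
; On BeginPlay it caches its grunt anim instance, then spawns a BP_GunParent and attaches it to the right-hand socket.
; Start and stop shooting events toggle aim state, the animation flag and walk speed, and forward to the gun.
; Entering cover crouches the character and has its AIC_Enemy controller run the BT_Commander behavior tree.
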(event Custom|StartShooting
  (Variables|Default|SetIsADS true)
  (Variables|/Game/Blueprints/AI/BP_RangedGrunt_AnimBP.BP_RangedGrunt_AnimBP_C|SetIsShooting (Variables|Default|GetAnimInstance) true)
  (Variables|/Script/Engine.CharacterMovementComponent|SetMaxWalkSpeed (Variables|Character|GetCharacterMovement) 2.7e+02)
  (Default|StartShooting (Variables|Default|GetBP_GUN)))

(event Custom|StopShooting
  (Variables|Default|SetIsADS false)
  (Variables|/Game/Blueprints/AI/BP_RangedGrunt_AnimBP.BP_RangedGrunt_AnimBP_C|SetIsShooting (Variables|Default|GetAnimInstance) false)
  (Variables|/Script/Engine.CharacterMovementComponent|SetMaxWalkSpeed (Variables|Character|GetCharacterMovement) 6e+02)
  (Default|StopShooting (Variables|Default|GetBP_GUN)))

(event Custom|SpawnWeapon
  ;[1 1 1] Spawn Rifle on Enemy AI to hand_rSocket and attach it to the actor component
  (bind _returnvalue (Game|SpawnActorfromClass "/Game/Blueprints/Weapons/Guns/BP_GunParent.BP_GunParent_C" (Transformation|GetSocketTransform (Variables|Character|GetMesh) "hand_rSocket" "RTS_World") "Undefined" 0 0))
  (bind _output_get (Variables|Default|SetBP_GUN _returnvalue))
  (Transformation|AttachComponentToComponent _output_get (Variables|Character|GetMesh) "hand_rSocket" "SnapToTarget" "SnapToTarget" "SnapToTarget" true))

(event Custom|EnterCover
  (Variables|Default|SetIsInCover true)
  (Character|Crouch)
  (bind _asaic_enemy (Utilities|Casting|CastToAIC_Enemy (AI|GetAIController 0)))
  (AI|RunBehaviorTree _asaic_enemy "/Game/Blueprints/AI/BT_Commander.BT_Commander"))

(event EventBeginPlay
  (bind _asbp_ranged_grunt_anim_bp (Utilities|Casting|CastToBP_RangedGrunt_AnimBP (Components|SkeletalMesh|GetAnimInstance (Variables|Character|GetMesh))))
  (Variables|Default|SetAnimInstance _asbp_ranged_grunt_anim_bp)
  (CallFunction|SpawnWeapon))

(fn ConstructionScript)