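; CH_Boss is a boss AI character that attacks targets and can leap at the player, using the ranged grunt's animation blueprint.
; Attack snaps yaw toward a valid target, then starts default attack 0 regardless of target validity.
; Launch computes a custom-arc velocity to player 0's pawn and launches the character with it.
; MissileBarrage is an empty stub, and an alternative projectile-velocity node is left unconnected.
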(event Custom|Launch
  (bind _outlaunchvelocity (Game|SuggestProjectileVelocityCustomArc (Transformation|GetActorLocation) (Transformation|GetActorLocation (Game|Player|GetPlayerPawn 0)) 0.0 0.7))
  (Character|LaunchCharacter _outlaunchvelocity true true))

(event Custom|MissileBarrage)

(event Custom|Attack
  (params (Target%20Actor :type Actor%20Object%20Reference))
  (Utilities|FlowControl|Sequence
    (:then_0
      (Utilities|IsValid Target%20Actor
        (:Is%20Valid
          (Transformation|SetActorRotation (Math|Rotator|MakeRotator 0.0 0.0 (.yaw (Math|Rotator|FindLookatRotation (Transformation|GetActorLocation) (Transformation|GetActorLocation Target%20Actor))))))))
    (:then_1
      (Class|CharacterInterface|StartDefaultAttack))))

(event EventBeginPlay
  (bind _asbp_ranged_grunt_anim_bp (Utilities|Casting|CastToBP_RangedGrunt_AnimBP (Components|SkeletalMesh|GetAnimInstance (Variables|Character|GetMesh))))
  (Variables|Default|SetAnimInstance _asbp_ranged_grunt_anim_bp))

(fn ConstructionScript)