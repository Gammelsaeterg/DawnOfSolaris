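; EncounterArea is an AI area actor that shares a called-out target location with the enemies inside it.
; Its CallOutTarget event stores the location, gathers every AIC_Enemy actor in the world and keeps those overlapping the area.
; It writes each one's TargetLocation blackboard key and sets HasLineOfSight to true, so they behave as if they see the target themselves.
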(event Custom|CallOutTarget
  (params (TargetLocation :type Vector))
  (Variables|Default|SetTargetLocation TargetLocation)
  (bind _outactors (Actor|GetAllActorsOfClass "/Game/Blueprints/AI/AIC_Enemy.AIC_Enemy_C"))
  (for _array_element _outactors
    (if (Collision|IsOverlappingActor _array_element :!class /Script/Engine.Actor)
      (AI|Components|Blackboard|SetValueasVector (AI|GetBlackboard _array_element) (Utilities|Name|MakeLiteralName "TargetLocation") (Variables|Default|GetTargetLocation))
      (AI|Components|Blackboard|SetValueasBool (AI|GetBlackboard _array_element) (Utilities|Name|MakeLiteralName "HasLineOfSight") true))))

(fn ConstructionScript)