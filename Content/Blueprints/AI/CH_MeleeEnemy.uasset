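; Melee enemy character Blueprint that supplies an attack action against a given target actor.
; The Attack event snaps the character's yaw toward the target if it is valid, then calls StartDefaultAttack with index zero whether or not the target is valid.
; BeginPlay, Tick and the construction script are empty, and a walk-speed debug print is left unconnected.
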(event Custom|Attack
  (params (Target%20Actor :type Actor%20Object%20Reference))
  (Utilities|FlowControl|Sequence
    (:then_0
      (Utilities|IsValid Target%20Actor
        (:Is%20Valid
          (Transformation|SetActorRotation (Math|Rotator|MakeRotator 0.0 0.0 (.yaw (Math|Rotator|FindLookatRotation (Transformation|GetActorLocation) (Transformation|GetActorLocation Target%20Actor))))))))
    (:then_1
      (Class|CharacterInterface|StartDefaultAttack))))

(event EventBeginPlay)

(event EventTick
  (params (DeltaSeconds :type Float%20%28single-precision%29)))

(fn ConstructionScript)