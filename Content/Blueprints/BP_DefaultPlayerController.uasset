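; Default player controller that handles target lock-on input and pause-menu flow for the alien player character.
; On BeginPlay it initializes TSComponent with AI perception and the pawn, then routes Target input to lock-on and left/right switching.
; CheckTargetingToggle and DisableTargeting update the character's IsTargeting flag.
; Pause input calls PauseGame, defined outside these graphs; Blueprint functions implement the pause widget, resume, level reset and quit to StartMenuMap.
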(event Custom|CheckTargetingToggle
  ;[0 0 0] Lock On To Target|Copy and Paste Into Your Own Blueprints If Desired
  (bind _controlledpawn (Variables|Default|GetControlledPawn)
    (:then
      (bind _asch_alien_player_character (Utilities|Casting|CastToCH_AlienPlayerCharacter _controlledpawn))
      (Variables|/Script/DawnOfSolaris.BaseCharacter|SetbIsTargeting _asch_alien_player_character (Variables|/Game/MarketplaceContent/TheTargetingSystem/_Component/TS.TS_C|GetIs%20Lock%20On%20Enabled? (Variables|Default|GetTS_component))))
    (:else)))

(event EventBeginPlay
  ;[0 0 0] Initialize Targeting System's Key Variables and Mechanics|Copy and Paste Into Your Own Blueprints If Desired
  (Default|InitializeVariables (Variables|Default|GetTS_component) (Variables|Default|GetAIPerception) (Pawn|GetControlledPawn self)))

(event EventPossess
  (params (PossessedPawn :type Pawn%20Object%20Reference))
  ;[0 0 0] Lock On To Target|Copy and Paste Into Your Own Blueprints If Desired
  (Variables|Default|SetControlledPawn PossessedPawn))

(event Input|ActionEvents|InputActionPause
  (params (Key :type Key%20Structure))
  (:Pressed
    (Class|DefaultPlayerController|PauseGame)))

(event Input|ActionEvents|InputActionTarget
  (params (Key :type Key%20Structure))
  ;[0 0 0] Lock On To Target|Copy and Paste Into Your Own Blueprints If Desired
  (:Pressed
    (Default|LockontoTarget (Variables|Default|GetTS_component))))

(event Input|ActionEvents|InputActionTargetLeft
  (params (Key :type Key%20Structure))
  ;[0 0 0] Lock On To Target|Copy and Paste Into Your Own Blueprints If Desired
  (:Pressed
    (Default|LockontoTargettotheLeft (Variables|Default|GetTS_component))))

(event Input|ActionEvents|InputActionTargetRight
  (params (Key :type Key%20Structure))
  ;[0 0 0] Lock On To Target|Copy and Paste Into Your Own Blueprints If Desired
  (:Pressed
    (Default|LockontoTargettotheRight (Variables|Default|GetTS_component))))

(fn ConstructionScript)

(fn PauseGameBP
  (bind _self self)
  (bind _returnvalue (UserInterface|CreateWidget "/Game/UI/UI_PauseMenu.UI_PauseMenu_C" self))
  (bind _output_get (Variables|Default|SetPauseMenuWidgetBP _returnvalue))
  (UserInterface|Viewport|AddtoViewport _output_get 0)
  (Variables|/Script/UMG.UserWidget|SetbIsFocusable (Variables|Default|GetPauseMenuWidgetBP) true)
  (Variables|/Script/Engine.PlayerController|SetbShowMouseCursor _self true)
  (Class|Widget|SetUserFocus (Variables|Default|GetPauseMenuWidgetBP) _self)
  (Game|SetGamePaused true))

(fn ContinueGameBP
  (bind _self self)
  (bind _pausemenuwidgetbp (Variables|Default|GetPauseMenuWidgetBP))
  (Game|SetGamePaused false)
  (Utilities|IsValid _pausemenuwidgetbp
    (:Is%20Valid
      (Widget|RemovefromParent _pausemenuwidgetbp))
    (:Is%20Not%20Valid
      _))
  (Variables|/Script/Engine.PlayerController|SetbShowMouseCursor _self false)
  (Input|SetInputModeGameOnly _self))

(fn ResetLevelBP
  (bind _returnvalue (Game|GetCurrentLevelName true))
  (CallFunction|ContinueGameBP)
  (Game|OpenLevel(byName) (Utilities|String|StringToName _returnvalue)))

(fn QuitGameBP
  (Game|OpenLevel(byName) "StartMenuMap"))

(fn DisableTargeting
  (bind _controlledpawn (Variables|Default|GetControlledPawn)
    (:then
      (bind _asch_alien_player_character (Utilities|Casting|CastToCH_AlienPlayerCharacter _controlledpawn))
      (Variables|/Script/DawnOfSolaris.BaseCharacter|SetbIsTargeting _asch_alien_player_character false))
    (:else)))