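; Anim notify state that plays an attached Niagara effect during part of an alien player character's animation.
; On begin it spawns the system inactive at a socket, then feeds it the notify duration, the character's current morph mesh and crystal color before activating it.
; The effect is stored on the character, and notify end deactivates it through that reference rather than through the notify's own variable.
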(fn ReceivedNotifyBegin
  (params (MeshComp :type Skeletal%20Mesh%20Component%20Object%20Reference) (Animation :type Anim%20Sequence%20Base%20Object%20Reference) (TotalDuration :type Float%20%28single-precision%29))
  (LocalVariables|SetTimeDuration TotalDuration)
  (bind _returnvalue (Niagara|SpawnSystemAttached (Variables|Default|GetParticle) MeshComp (Variables|Default|GetSocket%20Name) "0, 0, 0" "0, 0, 0" "KeepRelativeOffset" true false))
  (LocalVariables|SetCurrentParticle _returnvalue)
  (bind _asch_alien_player_character (Utilities|Casting|CastToCH_AlienPlayerCharacter (Components|GetOwner MeshComp))
    (:then
      (Variables|/Game/Blueprints/CH_AlienPlayerCharacter.CH_AlienPlayerCharacter_C|SetcurrentActiveMontageNiagaraParticle _asch_alien_player_character _returnvalue)
      (bind _currentmorphmesh (Default|GetCurrentMorphMesh _asch_alien_player_character))
      (Class|NiagaraFunctionLibrary|OverrideSystemUserVariableStaticMeshComponent (LocalVariables|GetCurrentParticle) "User.StaticMesh" _currentmorphmesh)
      (Effects|Components|ParticleSystem|SetFloatParameter (LocalVariables|GetCurrentParticle) "User.Duration" (LocalVariables|GetTimeDuration))
      (bind _color (Default|GetCurrentCrystalColor _asch_alien_player_character))
      (Niagara|SetNiagaraVariable(LinearColor) (LocalVariables|GetCurrentParticle) "User.CustomColor" _color))
    (:CastFailed
      _))
  (Components|Activation|Activate (LocalVariables|GetCurrentParticle) false)
  (return true))

(fn ReceivedNotifyEnd
  (params (MeshComp :type Skeletal%20Mesh%20Component%20Object%20Reference) (Animation :type Anim%20Sequence%20Base%20Object%20Reference))
  (bind _asch_alien_player_character (Utilities|Casting|CastToCH_AlienPlayerCharacter (Components|GetOwner MeshComp))
    (:then
      (bind _currentactivemontageniagaraparticle (Variables|/Game/Blueprints/CH_AlienPlayerCharacter.CH_AlienPlayerCharacter_C|GetcurrentActiveMontageNiagaraParticle _asch_alien_player_character)
        (:then
          (Components|Activation|Deactivate _currentactivemontageniagaraparticle))
        (:else
          _)))
    (:CastFailed
      _))
  (return true))