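; Animation notify state that plays a sound for the length of its window, used for the alien player character's charge audio.
; On begin, it spawns the sound attached to a mesh socket with slight random pitch and stores it in the character's CurrentChargeAudioComponent.
; On end, it briefly fades out that stored component if valid.
; Other owners still get the sound, but it is neither stored nor faded by the notify.
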(fn ReceivedNotifyBegin
  (params (MeshComp :type Skeletal%20Mesh%20Component%20Object%20Reference) (Animation :type Anim%20Sequence%20Base%20Object%20Reference) (TotalDuration :type Float%20%28single-precision%29))
  (bind _returnvalue (Audio|SpawnSoundAttached (Variables|Default|GetSoundToPlay) MeshComp (Variables|Default|GetSocket%20Name) "0, 0, 0" "0, 0, 0" (Variables|Default|GetAttachRules) false 1.0 (Math|Random|RandomFloatinRange 0.98 1.02) 0.0 "/Game/Sound/NewSoundAttenuation.NewSoundAttenuation" 0))
  (bind _asch_alien_player_character (Utilities|Casting|CastToCH_AlienPlayerCharacter (Components|GetOwner MeshComp)))
  (bind _output_get (Variables|/Game/Blueprints/CH_AlienPlayerCharacter.CH_AlienPlayerCharacter_C|SetCurrentChargeAudioComponent _asch_alien_player_character _returnvalue))
  (Audio|Components|Audio|Play _output_get 0.0)
  (return true))

(fn ReceivedNotifyEnd
  (params (MeshComp :type Skeletal%20Mesh%20Component%20Object%20Reference) (Animation :type Anim%20Sequence%20Base%20Object%20Reference))
  (bind _asch_alien_player_character (Utilities|Casting|CastToCH_AlienPlayerCharacter (Components|GetOwner MeshComp)))
  (bind _currentchargeaudiocomponent (Variables|/Game/Blueprints/CH_AlienPlayerCharacter.CH_AlienPlayerCharacter_C|GetCurrentChargeAudioComponent _asch_alien_player_character)
    (:then
      (Audio|Components|Audio|FadeOut _currentchargeaudiocomponent 0.2 0.0 "Linear" :!class /Script/Engine.AudioComponent)
      (return true))
    (:else)))