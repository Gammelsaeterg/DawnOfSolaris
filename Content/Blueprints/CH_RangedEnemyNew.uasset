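; CH_RangedEnemyNew is a ranged enemy Blueprint that adds optional appearance variation and timed cleanup to its parent class.
; On BeginPlay, if RandomizeAppearance is set, it randomizes scale independently per axis within configurable bounds and applies a slight random HueShift through a dynamic material instance on the mesh's first material slot.
; On defeat, it runs the parent's handling, then sets a one-minute lifespan so the actor removes itself.
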(event EventBeginPlay
  (bind _randomscalemin (Variables|Default|GetRandomScaleMin))
  (bind _randomscalemax (Variables|Default|GetRandomScaleMax))
  (bind _returnvalue (Math|Random|RandomFloatinRange _randomscalemin _randomscalemax))
  ;[1 1 1] Appearance randomizer
  (if (Variables|Default|GetbRandomizeAppearance)
    (Transformation|SetActorScale3D (Math|Vector|MakeVector _returnvalue _returnvalue _returnvalue))
    (bind _returnvalue_2 (Rendering|Material|CreateDynamicMaterialInstance (Variables|Character|GetMesh) 0 (Rendering|Material|GetMaterial (Variables|Character|GetMesh) 0) "None" :!class /Script/Engine.PrimitiveComponent))
    (Rendering|Material|SetScalarParameterValue _returnvalue_2 "HueShift" (Math|Random|RandomFloatinRange -0.065 0.065) :!class /Script/Engine.MaterialInstanceDynamic)))

(event EventEventIsDefeated
  ;[1 1 1] Appearance randomizer
  (|CallParentFunction)
  (Actor|SetLifeSpan 6e+01))

(fn ConstructionScript)