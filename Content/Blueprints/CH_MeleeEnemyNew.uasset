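; Melee enemy character Blueprint whose active logic only randomizes its appearance when play begins.
; If RandomizeAppearance is set, it rolls each scale axis independently and applies a slight random HueShift through a dynamic material instance on the mesh.
; Attack and Tick are empty; disconnected leftover nodes would turn the enemy toward TargetActor and start the default attack.
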(event Custom|Attack
  (params (Target%20Actor :type Actor%20Object%20Reference))
  ;[1 1 1] TODO(?): Probably no longer needed
)

(event EventBeginPlay
  (bind _randomscalemin (Variables|Default|GetRandomScaleMin))
  (bind _randomscalemax (Variables|Default|GetRandomScaleMax))
  (bind _returnvalue (Math|Random|RandomFloatinRange _randomscalemin _randomscalemax))
  ;[1 1 1] Appearance randomizer
  (if (Variables|Default|GetbRandomizeAppearance)
    (Transformation|SetActorScale3D (Math|Vector|MakeVector _returnvalue _returnvalue _returnvalue))
    (bind _returnvalue_2 (Rendering|Material|CreateDynamicMaterialInstance (Variables|Character|GetMesh) 0 (Rendering|Material|GetMaterial (Variables|Character|GetMesh) 0) "None" :!class /Script/Engine.PrimitiveComponent))
    (Rendering|Material|SetScalarParameterValue _returnvalue_2 "HueShift" (Math|Random|RandomFloatinRange -0.035 0.035) :!class /Script/Engine.MaterialInstanceDynamic)))

(event EventTick
  (params (DeltaSeconds :type Float%20%28single-precision%29)))

(fn ConstructionScript)