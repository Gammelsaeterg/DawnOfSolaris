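; Destructible crate or barrier that recoils when hit and fractures into physics debris when broken.
; A damage event offsets the base mesh along the hit direction, and Tick eases it home with VectorSpringInterp while not destroyed, using a fresh spring state each frame.
; The break event prints a debug message and calls FractureMesh, which hides the base mesh and reveals the simulated, collidable destructible mesh.
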(event EventBeginPlay
  (Collision|SetCollisionEnabled (Variables|Default|GetdestructibleMesh) "NoCollision")
  (bind _output_get (Variables|Default|SetInitialLocation (Transformation|GetWorldLocation (Variables|Default|GetbaseMesh))))
  (Variables|Default|SetNewDisplacement _output_get))

(event EventBreakBarrierBlueprintEvent
  (Development|PrintString "Barrier break" true true "(R=0.000000,G=0.660000,B=1.000000,A=1.000000)" 1e+01)
  (CallFunction|FractureMesh))

(event EventTick
  (params (DeltaSeconds :type Float%20%28single-precision%29))
  (if (not (Variables|Default|GetbIsDestroyed))
    (bind _returnvalue (Class|KismetMathLibrary|VectorSpringInterp (Variables|Default|GetNewDisplacement) (Variables|Default|GetInitialLocation) (Utilities|Struct|MakeVectorSpringState) 3e+01 0.5 DeltaSeconds 0.2))
    (Transformation|SetWorldLocation (Variables|Default|GetbaseMesh) _returnvalue false false)
    (Variables|Default|SetNewDisplacement _returnvalue)))

(event EventTakeDamageBlueprintEvent
  (params (hitDirection :type Vector :default "0, 0, 0"))
  (Variables|Default|SetNewDisplacement (+ (Variables|Default|GetInitialLocation) (* hitDirection 5e+01))))

(fn ConstructionScript)

(fn FractureMesh
  (bind _destructiblemesh (Variables|Default|GetdestructibleMesh))
  (Collision|SetCollisionEnabled (Variables|Default|GetbaseMesh) "NoCollision")
  (Rendering|SetVisibility (Variables|Default|GetbaseMesh) false false)
  (Rendering|SetVisibility (Variables|Default|GetdestructibleMesh) true false)
  (Physics|SetSimulatePhysics _destructiblemesh true)
  (Collision|SetCollisionEnabled _destructiblemesh "QueryAndPhysics")
  (Collision|SetCollisionResponsetoChannel _destructiblemesh "ECC_Pawn" "ECR_Block"))