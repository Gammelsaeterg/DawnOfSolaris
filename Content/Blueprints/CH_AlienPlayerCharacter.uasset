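; Alien player character that adds moveset-driven visuals, eye blinking and placeholder respawn-on-defeat.
; Dynamic crystal materials light up for the active moveset and supply colour to morph particles, eyes and hit bursts.
; Moveset changes briefly spawn the target weapon to copy its mesh, then feed current and next meshes into a Niagara morph effect.
; A looping timer drives the blink morph target, and defeat teleports to spawn with full health.
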(event Custom|StartBlinking
  ;[1 1 1] Eye blink
  (bind _blink (Timeline|BlinkTimeline PlayFromStart)
    (:Update
      (Components|SkeletalMesh|SetMorphTarget (Variables|Character|GetMesh) "Blink" _blink true))))

(event Custom|InitializeCrystalColors
  ;[0.1479 1 0] CrystalUpdate
  (CallFunction|UpdateCrystalMaterials (Variables|Default|GetcurrentMovesetIndex)))

(event EventBeginPlay
  ;[0.1447 1 0] BeginPlay
  (|CallParentFunction)
  (Variables|Default|SetRespawnLocation (Transformation|GetActorLocation))
  (CallFunction|InitializeCrystals)
  (Utilities|Time|SetTimerbyFunctionName self "StartBlinking" 5.0 true)
  (CallFunction|InitializeCrystalColors))

(event Collision|EventActorBeginOverlap
  (params (OtherActor :type Actor%20Object%20Reference))
  (|CallParentFunction OtherActor) ; This node is disabled and will not be called.\nDrag off pins to build functionality.
)

(event EventTick
  (params (DeltaSeconds :type Float%20%28single-precision%29))
  ;[0 1 0.06875] Tick
  (|CallParentFunction DeltaSeconds))

(event EventEventIsDefeated
  ;[1 1 1] DefeatProcedure, TODO: Expand as current blueprint data was made for playtesting
  (Transformation|SetActorLocation (Variables|Default|GetRespawnLocation) false false)
  (Variables|Default|SetcurrentHealthPoints (Variables|Default|GetmaxHealthPoints)))

(event EventDebugSpawnHitFX
  (params (hitLocation :type Vector :default "0, 0, 0"))
  ;[1 1 1] Hit FX
  (bind _returnvalue (Niagara|SpawnSystematLocation "/Game/Particles/Niagara/AlienBurst/NS_AlienBurst.NS_AlienBurst" hitLocation))
  (bind _color (CallFunction|GetCurrentCrystalColor))
  (Niagara|SetNiagaraVariable(LinearColor) _returnvalue "CustomColor" _color)
  (Audio|PlaySoundatLocation "/Game/Sound/PlaceholderSounds/whack1.whack1" hitLocation "0, 0, 0" (/ (Variables|/Script/DawnOfSolaris.MainGameInstance|GetsoundVolume (.AsBP%20Default%20Game%20Instance (Utilities|Casting|CastToBP_DefaultGameInstance (Game|GetGameInstance)))) 1e+02) (Math|Random|RandomFloatinRange 0.85 1.15) 0.0 "/Game/MigratedContent/MigratedAudio/LevelSoundAttenuation.LevelSoundAttenuation" 0 0))

(event EventEventStartChangeMoveset
  (params (nextMoveset :type Boolean))
  (bind _aliennextmorph (Variables|Default|GetAlienNextMorph))
  ;[0.1149 1 0] Morph particle procedure
  (if nextMoveset
    (bind _returnvalue (Class|PlayerCharacter|GetNextMoveset))
    (Variables|Default|SetnextMorphName (.movesetname _returnvalue))
    (bind _returnvalue_2 (Game|SpawnActorfromClass (.playerweaponmorph _returnvalue) (Math|Transform|MakeTransform "0, 0, 0") "Undefined" 0 0))
    (Components|StaticMesh|SetStaticMesh _aliennextmorph (Variables|/Script/Engine.StaticMeshComponent|GetStaticMesh (Variables|/Script/DawnOfSolaris.BaseWeapon|GetWeaponMesh _returnvalue_2)))
    (Actor|DestroyActor _returnvalue_2)
    (else
      (bind _returnvalue_3 (Class|PlayerCharacter|GetPreviousMoveset))
      (Variables|Default|SetnextMorphName (.movesetname _returnvalue_3))
      (bind _returnvalue_4 (Game|SpawnActorfromClass (.playerweaponmorph _returnvalue_3) (Math|Transform|MakeTransform "0, 0, 0") "Undefined" 0 0))
      (Components|StaticMesh|SetStaticMesh _aliennextmorph (Variables|/Script/Engine.StaticMeshComponent|GetStaticMesh (Variables|/Script/DawnOfSolaris.BaseWeapon|GetWeaponMesh _returnvalue_4)))
      (Actor|DestroyActor _returnvalue_4)))
  (bind _asbp_base_weapon (Utilities|Casting|CastToBP_BaseWeapon (Variables|/Script/Engine.ChildActorComponent|GetChildActor (Variables|Default|GetWeapon))))
  (Components|StaticMesh|SetStaticMesh (Variables|Default|GetAlienCurrentMorph) (Variables|/Script/Engine.StaticMeshComponent|GetStaticMesh (Variables|/Script/DawnOfSolaris.BaseWeapon|GetWeaponMesh _asbp_base_weapon)))
  (bind _returnvalue_5 (Niagara|SpawnSystemAttached "/Game/Particles/Niagara/Morph/NS_WeaponMorph.NS_WeaponMorph" (Variables|Default|GetWeapon) "lowerarm_l" "0, 0, 0" "0, 0, 0" "KeepWorldPosition" true false "AutoRelease"))
  (Class|NiagaraFunctionLibrary|OverrideSystemUserVariableStaticMeshComponent _returnvalue_5 "User.StartMesh" (Variables|Default|GetAlienCurrentMorph))
  (Class|NiagaraFunctionLibrary|OverrideSystemUserVariableStaticMeshComponent _returnvalue_5 "User.EndMesh" (Variables|Default|GetAlienNextMorph))
  (if (Variables|Default|GetbCrystalsInitialized)
    (switch string (Variables|Default|GetnextMorphName)
      (:AlienFists
        (Variables|Default|SetnextMorphIndex 0))
      (:AlienBlaster
        (Variables|Default|SetnextMorphIndex 1))
      (:AlienClub
        (Variables|Default|SetnextMorphIndex 2)))
    (bind _returnvalue_6 (Rendering|Material|GetVectorParameterValue (Utilities|Array|Get(acopy) (Variables|Default|GetCrystalMatInstances) (Utilities|Select :Index (Variables|Default|GetnextMorphIndex) :Option%200 0 :Option%201 1 :Option%202 3)) "EmissiveColor" :!class /Script/Engine.MaterialInstanceDynamic))
    (Niagara|SetNiagaraVariable(LinearColor) _returnvalue_5 "User.Color" _returnvalue_6))
  (Components|Activation|Activate _returnvalue_5 true)
  (Rendering|Material|SetVectorParameterValue (Variables|Default|GetEyesMatInstance) "Color" _returnvalue_6 :!class /Script/Engine.MaterialInstanceDynamic))

(event EventEventMovesetChanged
  ;[0.1479 1 0] CrystalUpdate
  (CallFunction|UpdateCrystalMaterials (Variables|Default|GetcurrentMovesetIndex)))

(event Input|KeyboardEvents|Q
  (params (Key :type Key%20Structure :default "None"))
  ;[1 1 1] Debug particle test
)

(fn ConstructionScript
  (|CallParentFunction))

(fn UpdateCrystalMaterials
  (params (inCrystalPowerIndex :type Integer))
  (bind _returnvalue (Utilities|Select :Index inCrystalPowerIndex :Option%200 0 :Option%201 1 :Option%202 3))
  (bind _crystalmatinstances (Variables|Default|GetCrystalMatInstances))
  (bind _output (Utilities|Array|Get(acopy) _crystalmatinstances _returnvalue))
  (if (Variables|Default|GetbCrystalsInitialized)
    (for _array_element (Variables|Default|GetCrystalMatInstances)
      (Rendering|Material|SetScalarParameterValue _array_element "EmissiveColorStrength" 0.0 :!class /Script/Engine.MaterialInstanceDynamic)
      (Rendering|Material|SetScalarParameterValue _output "EmissiveColorStrength" 1e+01 :!class /Script/Engine.MaterialInstanceDynamic)
      (Rendering|Material|SetMaterial (Variables|Character|GetMesh) 6 _output)
      (Rendering|Material|SetScalarParameterValue _output "Opacity" 1.0 :!class /Script/Engine.MaterialInstanceDynamic))))

(fn InitializeCrystals
  (bind _mesh (Variables|Character|GetMesh))
  (for _index (range 4 7)
    (bind _returnvalue (Rendering|Material|CreateDynamicMaterialInstance (Variables|Character|GetMesh) _index (Rendering|Material|GetMaterial (Variables|Character|GetMesh) _index) "None" :!class /Script/Engine.PrimitiveComponent))
    (Utilities|Array|Add (Variables|Default|GetCrystalMatInstances) _returnvalue)
    (Rendering|Material|SetScalarParameterValue _returnvalue "Opacity" 0.0 :!class /Script/Engine.MaterialInstanceDynamic)
    (bind _returnvalue_2 (Rendering|Material|CreateDynamicMaterialInstance _mesh 3 (Rendering|Material|GetMaterial _mesh 3) "None" :!class /Script/Engine.PrimitiveComponent))
    (Variables|Default|SetEyesMatInstance _returnvalue_2))
  (Variables|Default|SetbCrystalsInitialized true))

(fn GetCurrentCrystalColor
  (bind _returnvalue (Rendering|Material|GetVectorParameterValue (Utilities|Array|Get(acopy) (Variables|Default|GetCrystalMatInstances) (Utilities|Select :Index (Variables|Default|GetcurrentMovesetIndex) :Option%200 0 :Option%201 1 :Option%202 3)) "EmissiveColor" :!class /Script/Engine.MaterialInstanceDynamic))
  (return _returnvalue))