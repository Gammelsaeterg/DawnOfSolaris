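; Player character Blueprint that records its player controller ID on possession and can visualise attack hitboxes for debugging.
; When the debug flag is on, Tick checks whether an attack hitbox is active.
; A resettable DoOnce reveals the debug box for the current hand or foot once per activation.
; When the hitbox is inactive, all four boxes are hidden and the DoOnce resets.
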(event EventBeginPlay)

(event EventPossessed
  (params (NewController :type Controller%20Object%20Reference))
  ;[1 1 1] SetPlayerIndex
  (bind _asplayer_controller (Utilities|Casting|CastToPlayerController NewController))
  (Variables|Default|SetcurrentPlayerID (Class|GameplayStatics|GetPlayerControllerID _asplayer_controller)))

(event EventTick
  (params (DeltaSeconds :type Float%20%28single-precision%29))
  ;[1 1 1] Show debug hitboxes
  (if (Variables|Default|GetShowDebugHitboxes)
    (CallFunction|DrawDebugHitboxes)))

(event Collision|EventActorBeginOverlap
  (params (OtherActor :type Actor%20Object%20Reference)))

(event Custom|ResetDoOnceDebug
  (bind _rightfootdebugbox (Variables|Default|GetRightFootDebugBox))
  (bind _lefthanddebugbox (Variables|Default|GetLeftHandDebugBox))
  (bind _righthanddebugbox (Variables|Default|GetRightHandDebugBox))
  (bind _leftfootdebugbox (Variables|Default|GetLeftFootDebugBox))
  (bind _array (Utilities|Array|MakeArray _lefthanddebugbox _righthanddebugbox _leftfootdebugbox _rightfootdebugbox))
  ;[1 1 1] Debug hitbox
  (Utilities|FlowControl|DoOnce false) ; enters at Reset
)

(event Custom|DrawDebugHitboxes
  (bind _rightfootdebugbox (Variables|Default|GetRightFootDebugBox))
  (bind _lefthanddebugbox (Variables|Default|GetLeftHandDebugBox))
  (bind _righthanddebugbox (Variables|Default|GetRightHandDebugBox))
  (bind _leftfootdebugbox (Variables|Default|GetLeftFootDebugBox))
  (bind _array (Utilities|Array|MakeArray _lefthanddebugbox _righthanddebugbox _leftfootdebugbox _rightfootdebugbox))
  ;[1 1 1] Debug hitbox
  (if (Variables|Default|GetbAttackHitboxActive)
    (Utilities|FlowControl|DoOnce false
      (:Completed
        (switch Utilities|FlowControl|Switch|SwitchonEAttackHitboxType (Variables|Default|GetcurrentAttackHitboxType)
          (:LeftHand
            (Rendering|SetVisibility (Utilities|Array|Get(acopy) _array) true false))
          (:LeftFoot
            (Rendering|SetVisibility (Utilities|Array|Get(acopy) _array 2) true false))
          (:RightHand
            (Rendering|SetVisibility (Utilities|Array|Get(acopy) _array 1) true false))
          (:RightFoot
            (Rendering|SetVisibility (Utilities|Array|Get(acopy) _array 3) true false)))))
    (else
      (for _array_element (Utilities|Array|MakeArray (Variables|Default|GetLeftHandDebugBox) (Variables|Default|GetRightHandDebugBox) (Variables|Default|GetLeftFootDebugBox) (Variables|Default|GetRightFootDebugBox))
        (Rendering|SetVisibility _array_element false false))
      (CallFunction|ResetDoOnceDebug))))

(fn ConstructionScript)